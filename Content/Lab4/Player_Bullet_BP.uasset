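; Player bullet actor that deals damage on overlap to enemies and to other Bullet actors.
; Box overlap subtracts Damage from the target's Health, then hides the bullet and zeroes its own Health, which Tick detects to destroy it.
; Only Bullet hits also play a sound and spawn an explosion at the bullet's transform.
; The CheckDamage function is empty.
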(event `self.Box.OnComponentBeginOverlap`
  (params (OverlappedComponent :type "PrimitiveComponent Object Reference") (OtherActor :type "Actor Object Reference") (OtherComp :type "PrimitiveComponent Object Reference") (OtherBodyIndex :type Integer) (bFromSweep :type Boolean) (SweepResult :type "HitResult Structure (by ref)"))
  (bind _damage (`self.damage`))
  (bind _asenemy (cast `/Game/Lab4/enemy` OtherActor)
    (:`then`
      (set `/Game/Lab4/enemy.health` (- (`/Game/Lab4/enemy.health` _asenemy) _damage) _asenemy)
      (`self.SetActorHiddenInGame` true)
      (set `self.health` 0))
    (:`CastFailed`
      (bind _asbullet (cast `/Game/ThirdPersonBP/Blueprints/Bullet` OtherActor))
      (`|ExecutionSequence`
        (:`then_0`
          (set `/Game/ThirdPersonBP/Blueprints/Bullet.health` (- (`/Game/ThirdPersonBP/Blueprints/Bullet.health` _asbullet) _damage) _asbullet)
          (`self.SetActorHiddenInGame` true)
          (set `self.health` 0))
        (:`then_1`
          (`GameplayStatics.PlaySound2D` "/Game/Lab4/music/mixkit-quick-jump-arcade-game-239.mixkit-quick-jump-arcade-game-239" 1.0 1.0 0.0 null null)
          (`|SpawnActorFromClass` "/Game/Lab4/music/Exxxxplosion.Exxxxplosion_C" (`self.GetTransform`) "Undefined" "OverrideRootScale" null null))))))

(event `self.ReceiveTick`
  (params (DeltaSeconds :type "Float (single-precision)"))
  (if (<= (`self.health`) 0)
    (`|ExecutionSequence`
      (:`then_0`
        (`self.K2_DestroyActor`)))))

(fn `Check damage`)

(fn `UserConstructionScript`)