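; Player bullet Blueprint that damages enemies on contact and then removes itself.
; Its box overlap subtracts Damage from an enemy's Health, then hides the bullet and zeroes its own Health.
; Overlapping another Bullet only hides and zeroes this one, and Tick destroys it once Health is depleted.
; Bullet-to-bullet damage, explosion and sound nodes are disconnected, and CheckDamage is empty.
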(event `self.Box.OnComponentBeginOverlap`
  (params (OverlappedComponent :type "PrimitiveComponent Object Reference") (OtherActor :type "Actor Object Reference") (OtherComp :type "PrimitiveComponent Object Reference") (OtherBodyIndex :type Integer) (bFromSweep :type Boolean) (SweepResult :type "HitResult Structure (by ref)"))
  (bind _asenemy (cast `/Game/Lab4/Logic/enemy` OtherActor)
    (:`then`
      (set `/Game/Lab4/Logic/enemy.health` (- (`/Game/Lab4/Logic/enemy.health` _asenemy) (`self.damage`)) _asenemy)
      (`self.SetActorHiddenInGame` true)
      (set `self.health` 0))
    (:`CastFailed`
      (bind _asbullet (cast `/Game/Lab4/Logic/Bullet` OtherActor))
      (`self.SetActorHiddenInGame` true)
      (set `self.health` 0))))

(event `self.ReceiveTick`
  (params (DeltaSeconds :type "Float (single-precision)"))
  (if (<= (`self.health`) 0)
    (`|ExecutionSequence`
      (:`then_0`
        (`self.K2_DestroyActor`)))))

(fn `Check damage`)

(fn `UserConstructionScript`)